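; BP_Enemy is an NPC enemy character that ragdolls and flies back when hit.
; Its Hit function disables movement, turns on mesh physics and switches off capsule collision.
; It then launches the mesh with a fixed-strength impulse along the hit direction tilted upward, spawns the NS_Hit Niagara effect and returns true.
; The Damage input is unused, so any hit triggers this reaction, and the event graph is empty.
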(event EventBeginPlay)

(event Collision|EventActorBeginOverlap
  (params (OtherActor :type Actor%20Object%20Reference)))

(event EventTick
  (params (DeltaSeconds :type Float%20%28single-precision%29)))

(fn ConstructionScript)

(fn Hit
  (params (Direction :type Vector :default "0, 0, 0") (Damage :type Integer))
  (bind _mesh (Variables|Character|GetMesh))
  (Pawn|Components|CharacterMovement|DisableMovement (Variables|Character|GetCharacterMovement))
  (Physics|SetSimulatePhysics _mesh true)
  (Collision|SetCollisionEnabled (Variables|Collision|GetCapsuleComponent) "NoCollision")
  (Collision|SetCollisionEnabled (Variables|Default|GetCapsule) "NoCollision")
  (Physics|AddImpulse _mesh (* (Math|Vector|Normalize (Math|Vector|Lerp(Vector) Direction (Transformation|GetActorUpVector) 0.3)) 1e+05) "None" false)
  (Niagara|SpawnSystematLocation "/Game/NS_Hit.NS_Hit" (Transformation|GetActorLocation))
  (return true))