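; Throwable player ladder actor that is launched by charge time, bounces off tagged surfaces and destroys itself when caught.
; Its physics collider takes the throw impulse and a scaled custom gravity force each tick.
; Overlaps with "BounceHorizontal" actors push it along its negated forward vector, briefly debounced, and store that force as CatchTransferForce until speed drops too low.
; Falling below a height limit kills the player character.
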(event Custom|Throw
  (params (Direction :type Vector) (Throw%20Charge%20Time :type Float%20%28double-precision%29))
  (Physics|AddImpulse (Variables|Default|GetLadderCollider) (* Direction (* Throw%20Charge%20Time (Variables|Default|GetThrow%20Force%20Scale))) "None" true))

(event Custom|Catch
  (Actor|DestroyActor))

(event EventTick
  (params (DeltaSeconds :type Float%20%28single-precision%29))
  (bind _returnvalue (Transformation|GetActorUpVector))
  (bind _returnvalue_2 (Transformation|GetActorForwardVector))
  (bind _bounce_force (Variables|Default|GetBounce%20Force))
  (bind _returnvalue_3 (Math|Vector|NegateVector _returnvalue_2))
  (bind _returnvalue_4 (Math|Vector|Lerp(Vector) _returnvalue_3 _returnvalue 0.0))
  (bind _returnvalue_5 (Math|Vector|Normalize _returnvalue_4))
  (bind _returnvalue_6 (* _returnvalue_5 _bounce_force))
  (Variables|Default|SetTime%20Since%20Bounce (+ (Variables|Default|GetTime%20Since%20Bounce) DeltaSeconds))
  (Physics|AddForce (Variables|Default|GetLadderCollider) (Math|Vector|MakeVector 0.0 0.0 (* (Variables|Default|GetGravity%20Scale) -9.8e+02)) "None" true)
  (if (< (.Z (Math|Vector|BreakVector (Transformation|GetActorLocation))) -2e+03)
    (bind _asbp_first_person_character (Utilities|Casting|CastToBP_FirstPersonCharacter (Game|GetPlayerCharacter 0)))
    (Default|Die _asbp_first_person_character)
    (else
      (bind _array_element (Utilities|Array|ForEachLoopwithBreak (Collision|GetOverlappingActors (Variables|Default|GetLarge%20Collider) 0 :!class /Script/Engine.PrimitiveComponent) :!label _label)
        (:LoopBody
          (if (and (> (Variables|Default|GetTime%20Since%20Bounce) 0.1) (Actor|ActorHasTag _array_element "BounceHorizontal"))
            (Physics|AddImpulse (Variables|Default|GetLadderCollider) _returnvalue_6 "None" true)
            (Variables|Default|SetCatch%20Transfer%20Force _returnvalue_6)
            (Variables|Default|SetTime%20Since%20Bounce 0.0)
            (goto _label Break)))
        (:Completed
          (if (< (Math|Vector|VectorLength (Transformation|GetComponentVelocity (Variables|Default|GetLadderCollider))) (Variables|Default|GetMin%20Speed%20For%20Catch))
            (Variables|Default|SetCatch%20Transfer%20Force "0, 0, 0")))))))

(fn ConstructionScript)