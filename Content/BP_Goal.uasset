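; BP_Goal is an actor, named as a goal, that floats and spins in place.
; BeginPlay stores its start location and resets a time counter.
; Each Tick adds a local rotation on all three axes, pitching twice as fast, and sets its height from a sine wave around the start location for a bobbing motion.
; It has no active overlap or goal-reaching logic.
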(event EventBeginPlay
  (Variables|Default|Settime 0.0)
  (Variables|Default|Setstart%20loc (Transformation|GetActorLocation)))

(event Collision|EventActorBeginOverlap
  (params (OtherActor :type Actor%20Object%20Reference)))

(event EventTick
  (params (DeltaSeconds :type Float%20%28single-precision%29))
  (bind _returnvalue (* DeltaSeconds 1e+01))
  (Transformation|AddActorLocalRotation (Math|Rotator|MakeRotator _returnvalue (* _returnvalue 2.0) _returnvalue) false false)
  (Variables|Default|Settime (+ (Variables|Default|Gettime) DeltaSeconds))
  (Transformation|SetActorLocation (+ (Variables|Default|Getstart%20loc) (* "0.000000,0.000000,1.000000" (* (Math|Trig|Sin(Radians) (* (Variables|Default|Gettime) 1.5)) 5e+01))) false false))

(fn ConstructionScript)