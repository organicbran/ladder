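; BP_HittableObject is a physics prop that gets knocked away when hit.
; Hit blends the incoming direction toward the actor's up vector, normalizes it and scales it by HitForce.
; It applies this to Cube as a mass-independent velocity-change impulse at a point offset from the actor's location.
; It then spawns the NS_Hit effect and returns true, ignoring Damage.
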(event EventBeginPlay)

(event Collision|EventActorBeginOverlap
  (params (OtherActor :type Actor%20Object%20Reference)))

(event EventTick
  (params (DeltaSeconds :type Float%20%28single-precision%29)))

(fn ConstructionScript)

(fn Hit
  (params (Direction :type Vector :default "0, 0, 0") (Damage :type Integer))
  (bind _returnvalue (Transformation|GetActorLocation))
  (Class|PrimitiveComponent|AddVelocityChangeImpulseatLocation (Variables|Default|GetCube) (* (Math|Vector|Normalize (Math|Vector|Lerp(Vector) Direction (Transformation|GetActorUpVector) 0.4)) (Variables|Default|GetHit%20Force)) (+ _returnvalue "0.000000,-20.000000,0.000000") "None")
  (Niagara|SpawnSystematLocation "/Game/NS_Hit.NS_Hit" _returnvalue)
  (return true))